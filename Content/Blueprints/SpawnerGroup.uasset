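; SpawnerGroup groups a set of spawners and hands out spawn positions from them on request.
; GetRandomSpawnPoint asks a random spawner for its position, while GetOrderedSpawnPoint cycles through the Spawners array with a wrapping Iterator.
; Both functions return the zero vector when the array is empty.
; It has no active event or construction logic, so it only responds to calls.
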(event EventBeginPlay)

(event Collision|EventActorBeginOverlap
  (params (OtherActor :type Actor%20Object%20Reference)))

(event EventTick
  (params (DeltaSeconds :type Float%20%28single-precision%29)))

(fn ConstructionScript)

(fn GetRandomSpawnPoint
  (bind _spawners (Variables|Default|GetSpawners))
  (if (== (Utilities|Array|Length _spawners) 0)
    (return (Math|Vector|MakeVector 0.0 0.0 0.0))
    (else
      (bind _point (Default|GetSpawnPos (.OutItem (Utilities|Array|Random _spawners))))
      (return _point))))

(fn GetOrderedSpawnPoint
  (bind _spawners (Variables|Default|GetSpawners))
  (bind _returnvalue (Utilities|Array|Length _spawners))
  (if (== _returnvalue 0)
    (return "0, 0, 0")
    (else
      (bind _result (Math|Integer|IncrementInt (Variables|Default|Getiterator))
        (:%20%20
          (if (>= _result _returnvalue)
            (Variables|Default|Setiterator 0))
          (bind _point (Default|GetSpawnPos (Utilities|Array|Get(acopy) _spawners (Variables|Default|Getiterator))))
          (return _point))))))